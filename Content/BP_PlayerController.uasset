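; Player controller that handles the bomb ability, its HUD icon and the player's death and respawn.
; On BeginPlay it adds a UI_Bomb widget to the viewport.
; Space bar calls UseBomb and swaps the icon to its used state, with a DoOnce reset after a short delay acting as the cooldown.
; KillPawn calls DyingPawn, waits, then calls RespawnPawn.
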(event Custom|KillPawn
  (Class|MyBombermanPlayerController|DyingPawn)
  (Utilities|FlowControl|Delay 15.0)
  (Class|MyBombermanPlayerController|RespawnPawn))

(event EventBeginPlay
  (bind _returnvalue (UserInterface|CreateWidget "/Game/UI_Bomb.UI_Bomb_C"))
  (bind _output_get (Variables|Default|SetBombIcon _returnvalue))
  (UserInterface|Viewport|AddtoViewport _output_get 0))

(event EventTick
  (params (DeltaSeconds :type Float%20%28single-precision%29)))

(event Input|KeyboardEvents|SpaceBar
  (params (Key :type Key%20Structure :default "None"))
  (:Pressed
    (Utilities|FlowControl|DoOnce false :!label _label
      (:Completed
        (Class|MyBombermanPlayerController|UseBomb "/Game/Bomb.Bomb")
        (Default|GetIcon (Variables|Default|GetBombIcon) (Variables|Default|GetIconUsedBomb))
        (Utilities|FlowControl|Delay 5.2)
        (Default|GetIcon (Variables|Default|GetBombIcon) (Variables|Default|GetIconBomb))
        (goto _label Reset)))))

(fn ConstructionScript)